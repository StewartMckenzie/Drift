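; Gameplay Ability that lets the hero sprint while the input is held.
; On activation it applies the GE_Sprint effect at the ability level and tells DriftCharacterMovementComponent to start sprinting.
; Releasing the input ends the ability, which removes the stored effect handle and stops sprinting on the movement component.
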(event Ability|EventActivateAbility
  (bind _returnvalue (Ability|ApplyGameplayEffectToOwner "/Game/Drift/Characters/Hero/Abilities/GE_Sprint.GE_Sprint_C" (Ability|GetAbilityLevel)))
  (Variables|Default|SetGESprint _returnvalue)
  (bind _asdrift_character_movement_component (Utilities|Casting|CastToDriftCharacterMovementComponent (.MovementComponent (Utilities|Struct|BreakGameplayAbilityActorInfo (Ability|GetActorInfo)))))
  (Class|DriftCharacterMovementComponent|StartSprinting _asdrift_character_movement_component)
  (Ability|Tasks|WaitInputRelease false
    (:OnRelease
      (Ability|EndAbility))))

(event Ability|EventOnEndAbility
  (params (bWasCancelled :type Boolean))
  (Ability|RemoveGameplayEffectFromOwnerWithHandle (Variables|Default|GetGESprint))
  (bind _asdrift_character_movement_component (Utilities|Casting|CastToDriftCharacterMovementComponent (.MovementComponent (Utilities|Struct|BreakGameplayAbilityActorInfo (Ability|GetActorInfo)))))
  (Class|DriftCharacterMovementComponent|StopSprinting _asdrift_character_movement_component))