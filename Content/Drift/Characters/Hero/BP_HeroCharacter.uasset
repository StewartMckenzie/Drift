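; Hero character Blueprint with target-lock, free-aim melee combos and a dynamic camera boom offset.
; Sphere traces along camera or movement direction pick a Target, falling back to the nearest; lock-on supports swapping, camera tracking, custom-depth highlighting and line-of-sight checks.
; Attacks cycle three-step montages with buffered input, using motion-warped dashes within range.
; The Timeline update that feeds line-of-sight checks and the camera-tracking gate is marked never run.
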(event Custom|ComboAttackSave
  (if (Variables|Default|GetSaveAttack)
    (Variables|Default|SetSaveAttack false)
    (if (Variables|Default|GetHasTarget) ; Check if we have a target
      (bind _returnvalue (CallFunction|CheckifinMotionWarpRange))
      (if _returnvalue
        (CallFunction|MotionWarpAttackTarget)
        (else
          (CallFunction|AttackinDirectionOfTarget)))
      (else
        (CallFunction|AttackinCameraDirection)))))

(event Custom|BreakLineOfSight
  (bind _returnvalue (Transformation|GetActorLocation))
  ;[1 1 1] TargetLock
  (if (Variables|Default|GetTargetLocked)
    (bind (_outhits _returnvalue_2) (Collision|MultiSphereTraceForObjects _returnvalue (+ _returnvalue "0,0.000000,0.100000") (Variables|Default|GetMaxTargetDistance) (Variables|Default|GetObject%20TypesArray) false 0 "None"))
    (if _returnvalue_2
      (for _array_element _outhits
        (if (not (== (.HitActor (Collision|BreakHitResult _array_element)) (Variables|Default|Gettarget)))
          (bind _astarget (Utilities|Casting|CastToTarget (.HitActor (Collision|BreakHitResult _array_element))))
          (Utilities|Array|Add (Variables|Default|GetIgnoreTargets) _astarget)))
      (CallFunction|SetHeadLocation)
      (bind (_outhit _returnvalue_3) (Collision|LineTraceForObjects (Variables|Default|GetHeadLocation) (Transformation|GetActorLocation (Variables|Default|Gettarget)) (Utilities|Array|MakeArray "ObjectTypeQuery1" "ObjectTypeQuery2" "ObjectTypeQuery7") false (Variables|Default|GetIgnoreTargets) "None"))
      (if _returnvalue_3
        (if (== (.hitactor _outhit) (Variables|Default|Gettarget)) :!label _label
          (Utilities|FlowControl|RetriggerableDelay 0.2)
          (if (Variables|Default|GetTargetSwapped)
            (Utilities|Array|Clear (Variables|Default|GetIgnoreTargets))
            (Variables|Default|SetTargetSwapped false)
            (else
              (Utilities|Array|Clear (Variables|Default|GetIgnoreTargets))
              (CallFunction|LockOff :!label _label_2)))
          (else
            (Utilities|FlowControl|Delay 5.0)
            (Utilities|Casting|CastToTargetPoint (.hitactor _outhit)
              (:then
                (Utilities|Array|Clear (Variables|Default|GetIgnoreTargets))
                (if (Variables|Default|GetTargetSwapped)
                  (Variables|Default|SetTargetSwapped false)
                  (goto _label)
                  (else
                    (goto _label_2))))
              (:CastFailed
                (goto _label_2))))))
      (else
        (goto _label_2)))))

(event Custom|LockOff
  ;[1 1 1] TargetLock
  (if (Variables|Default|GetTargetLocked)
    (CallFunction|ResetTargetingValues)
    (Utilities|FlowControl|Gate true) ; enters at Toggle
  ))

(event Custom|DynamicCamera
  (bind _boomanchor (Variables|Default|GetBoomAnchor))
  (bind _capsulecomponent (Variables|Default|GetCapsuleComponent))
  (bind _followcamera (Variables|Default|GetFollowCamera))
  (bind _returnvalue (Transformation|GetWorldLocation _boomanchor))
  (bind _returnvalue_2 (Transformation|GetWorldTransform _followcamera))
  (bind _returnvalue_3 (Transformation|GetWorldTransform _capsulecomponent))
  (bind _returnvalue_4 (- (.yaw (.rotation _returnvalue_3)) (.yaw (.rotation _returnvalue_2))))
  (bind _returnvalue_5 (+ _returnvalue_4 3.6e+02))
  (bind _returnvalue_6 (< _returnvalue_4 0.0))
  (bind _returnvalue_7 (Math|Float|SelectFloat _returnvalue_5 _returnvalue_4 _returnvalue_6))
  (bind _returnvalue_8 (< 1.8e+02 _returnvalue_7))
  (bind _returnvalue_9 (- _returnvalue_7 3.6e+02))
  (bind _returnvalue_10 (Math|Float|SelectFloat _returnvalue_9 _returnvalue_7 _returnvalue_8))
  (Transformation|SetWorldLocation (Variables|Default|GetCameraBoom) (.location (Class|KismetMathLibrary|TInterpto (Math|Transform|MakeTransform _returnvalue "0, 0, 0" "1,1,1") (Math|Transform|MakeTransform (+ _returnvalue (+ (+ (* (Math|Float|SelectFloat (* _returnvalue_10 -1.0) _returnvalue_10 (< _returnvalue_10 0.0)) (Math|Vector|GetForwardVector _boomanchor)) (Math|Vector|ClampVectorSize (* (Math|Vector|GetRightVector _boomanchor) (* (+ (Math|Float|SelectFloat (Math|Float|SelectFloat (- _returnvalue_10 (* (- _returnvalue_10 9e+01) 2.0)) _returnvalue_10 (< 9e+01 _returnvalue_10)) (Math|Float|SelectFloat (- _returnvalue_10 (* (+ _returnvalue_10 9e+01) 2.0)) _returnvalue_10 (< _returnvalue_10 -9e+01)) (< 0.0 _returnvalue_10)) 2e+01) 2.0)) 0.0 8e+01)) (* (Math|Vector|GetForwardVector (Variables|Default|GetBoomAnchor)) (* (* (.pitch (.rotation (Transformation|GetWorldTransform (Variables|Default|GetFollowCamera)))) -1.0) 0.75)))) "0, 0, 0" "1,1,1") (Utilities|Time|GetWorldDeltaSeconds) 0.0)) false false))

(event Custom|ResetCombo
  (Variables|Default|SetAttackCount 0)
  (Variables|Default|SetSaveAttack false)
  (Variables|Default|SetIsAttacking false))

(event Input|ActionEvents|InputActionTargetLock
  (params (Key :type Key%20Structure :default "None"))
  ;[1 1 1] TargetLock
  (:Pressed
    (CallFunction|SetHeadLocation)
    (if (Variables|Default|GetTargetLocked)
      (bind (_attackdirection _endoftrace) (CallFunction|GetCameraTraceValues (Variables|Default|GetMaxTargetDistance)))
      (Variables|Default|SetAttackDirection _attackdirection)
      (bind (_outhit _returnvalue) (Collision|SphereTraceForObjects (Variables|Default|GetHeadLocation) _endoftrace (Variables|Default|GetTargetLockTraceSize) (Variables|Default|GetObject%20TypesArray) false (Utilities|Array|MakeArray (Variables|Default|Gettarget)) "None"))
      (if _returnvalue
        (if (== (.hitactor _outhit) (Variables|Default|Gettarget))
          (CallFunction|ResetTargetingValues :!label _label)
          (Utilities|FlowControl|Gate true) ; enters at Toggle
          (else
            (bind _astarget (Utilities|Casting|CastToTarget (.hitactor _outhit))
              (:then
                (Variables|Default|SetTargetSwapped true)
                (bind _asbp_red_enemy (Utilities|Casting|CastToBP_RedEnemy (Actor|GetParentActor (Variables|Default|Gettarget))))
                (Rendering|SetRenderCustomDepth (Variables|/Script/Engine.Character|GetMesh _asbp_red_enemy) false)
                (Variables|Default|Settarget _astarget))
              (:CastFailed
                (CallFunction|ResetTargetingValues)))))
        (else
          (goto _label)))
      (else
        (bind (_attackdirection_2 _endoftrace_2) (CallFunction|GetCameraTraceValues (Variables|Default|GetMaxTargetDistance)))
        (CallFunction|DirectionalSingleTargetTrace _attackdirection_2 (Variables|Default|GetHeadLocation) _endoftrace_2 (Variables|Default|GetTargetLockTraceSize))
        (if (Variables|Default|GetHasTarget)
          (Variables|Default|SetTargetLocked true)
          (Utilities|FlowControl|Gate true) ; enters at Toggle
        )))))

(event Input|MouseEvents|LeftMouseButton
  (params (Key :type Key%20Structure :default "None"))
  (:Pressed
    (if (Variables|Default|GetTargetLocked)
      _
      (else
        (CallFunction|SetHeadLocation)
        (bind (_moving_ _movementdirection) (CallFunction|MovementDirectionCheck))
        (if _moving_ ; Check if I am standign still
          (bind (_attackdirection _endoftrace) (CallFunction|GetMovementTraceValues _movementdirection))
          (CallFunction|DirectionalSingleTargetTrace _attackdirection (Variables|Default|GetHeadLocation) _endoftrace (Variables|Default|GetFreeTraceSize))
          (else
            (bind (_attackdirection_2 _endoftrace_2) (CallFunction|GetCameraTraceValues (Variables|Default|GetMaxAttackDistance)))
            (CallFunction|DirectionalSingleTargetTrace _attackdirection_2 (Variables|Default|GetHeadLocation) _endoftrace_2 (Variables|Default|GetFreeTraceSize))))
        (if (Variables|Default|GetHasTarget)
          _
          (else
            (CallFunction|SphereMultiTargetTrace)))))
    (if (Variables|Default|GetIsAttacking)
      (Variables|Default|SetSaveAttack true)
      (else
        (Variables|Default|SetIsAttacking true)
        (if (Variables|Default|GetHasTarget) ; Check if we have a target
          (bind _returnvalue (CallFunction|CheckifinMotionWarpRange))
          (if _returnvalue
            (CallFunction|MotionWarpAttackTarget)
            (else
              (CallFunction|AttackinDirectionOfTarget)))
          (else
            (CallFunction|AttackinCameraDirection)))))))

(event Input|GamepadEvents|GamepadFaceButtonLeft
  (params (Key :type Key%20Structure :default "None"))
  (:Pressed
    (if (Variables|Default|GetTargetLocked)
      _
      (else
        (CallFunction|SetHeadLocation)
        (bind (_moving_ _movementdirection) (CallFunction|MovementDirectionCheck))
        (if _moving_ ; Check if I am standign still
          (bind (_attackdirection _endoftrace) (CallFunction|GetMovementTraceValues _movementdirection))
          (CallFunction|DirectionalSingleTargetTrace _attackdirection (Variables|Default|GetHeadLocation) _endoftrace (Variables|Default|GetFreeTraceSize))
          (else
            (bind (_attackdirection_2 _endoftrace_2) (CallFunction|GetCameraTraceValues (Variables|Default|GetMaxAttackDistance)))
            (CallFunction|DirectionalSingleTargetTrace _attackdirection_2 (Variables|Default|GetHeadLocation) _endoftrace_2 (Variables|Default|GetFreeTraceSize))))
        (if (Variables|Default|GetHasTarget)
          _
          (else
            (CallFunction|SphereMultiTargetTrace)))))
    (if (Variables|Default|GetIsAttacking)
      (Variables|Default|SetSaveAttack true)
      (else
        (Variables|Default|SetIsAttacking true)
        (if (Variables|Default|GetHasTarget) ; Check if we have a target
          (bind _returnvalue (CallFunction|CheckifinMotionWarpRange))
          (if _returnvalue
            (CallFunction|MotionWarpAttackTarget)
            (else
              (CallFunction|AttackinDirectionOfTarget)))
          (else
            (CallFunction|AttackinCameraDirection)))))))

(fn ConstructionScript)

(fn DirectionalSingleTargetTrace
  (params (AttackDriection :type Rotator) (Start%20of%20Trace :type Vector) (End%20of%20Trace :type Vector) (Radius%20of%20Trace :type Float%20%28single-precision%29))
  (Variables|Default|SetAttackDirection AttackDriection)
  (bind (_outhit _returnvalue) (Collision|SphereTraceForObjects Start%20of%20Trace End%20of%20Trace Radius%20of%20Trace (Variables|Default|GetObject%20TypesArray) false 0 "None"))
  (bind _astarget (Utilities|Casting|CastToTarget (.hitactor _outhit))
    (:then
      (Variables|Default|Settarget _astarget)
      (Variables|Default|SetHasTarget _returnvalue))
    (:CastFailed
      (Development|PrintString "Failed to cast to Target BP clss")))
  (return))

(fn SetHeadLocation
  (Variables|Default|SetHeadLocation (Transformation|GetWorldLocation (Variables|Default|GetCameraBoom)))
  (return))

(fn GetCameraTraceValues
  (params (TraceDistance :type Float%20%28single-precision%29))
  (bind _followcamera (Variables|Default|GetFollowCamera))
  (bind _returnvalue (Transformation|GetWorldRotation _followcamera))
  ;[1 1 1] If I am standing still start the trace on my head and have it extend the MaxTargetDistance in the direction my camera is looking
  (return _returnvalue (+ (* _returnvalue TraceDistance) (Variables|Default|GetHeadLocation))))

(fn GetMovementTraceValues
  (params (MovementVector :type Vector))
  ;[1 1 1] If I am standing still start the trace on my head and have it extend the MaxTargetDistance in the direction of my movement
  (return (Math|Conversions|RotationFromXVector MovementVector) (+ (Variables|Default|GetHeadLocation) (* (Math|Vector|Normalize MovementVector) (Variables|Default|GetMaxAttackDistance)))))

(fn MovementDirectionCheck
  (bind _charactermovement (Variables|Character|GetCharacterMovement))
  (bind _returnvalue (Pawn|Components|PawnMovement|GetLastInputVector _charactermovement))
  ;[1 1 1] Check if I am standing still
  (return (Utilities|Operators|NotEqual(!=) :A _returnvalue) _returnvalue))

(fn SphereMultiTargetTrace
  (bind _returnvalue (Transformation|GetActorLocation))
  ;[1 1 1] If I dont hit something sphere trace using my pawn's location as the center and my maxtargetDistance as the radius.
  (bind _outhits (Collision|MultiSphereTraceForObjects _returnvalue (+ _returnvalue "0,0.000000,0.100000") (Variables|Default|GetMaxAttackDistance) (Variables|Default|GetObject%20TypesArray) false 0 "None"))
  ;[1 1 1] Loop over everything hit comparing the distance of our current target to the previous target. If the current target is closer set ClosestTarget to the current distance, set this target object as our Target, and update HasTarget to true. If we hit nothing do nothing
  (for _array_element _outhits
    (if (< (Math|Vector|Distance(Vector) (Transformation|GetActorLocation (.HitActor (Collision|BreakHitResult _array_element))) (Transformation|GetActorLocation)) (Variables|Default|GetclosestTarget))
      (bind _astarget (Utilities|Casting|CastToTarget (.HitActor (Collision|BreakHitResult _array_element)))
        (:then
          (Variables|Default|SetclosestTarget (Math|Vector|Distance(Vector) (Transformation|GetActorLocation (.HitActor (Collision|BreakHitResult _array_element))) (Transformation|GetActorLocation)))
          (Variables|Default|Settarget _astarget)
          (Variables|Default|SetHasTarget true))
        (:CastFailed
          (Development|PrintString "Cast to target bp class failed"))))))

(fn CheckifinMotionWarpRange
  (Variables|Default|SetTargetLocation (Transformation|GetActorLocation (Variables|Default|Gettarget)))
  (Variables|Default|SetCharacterLocation (Transformation|GetActorLocation))
  (return (and (< (Math|Vector|Distance(Vector) (Variables|Default|GetTargetLocation) (Variables|Default|GetCharacterLocation)) (Variables|Default|GetMaxAttackDistance)) (> (Math|Vector|Distance(Vector) (Variables|Default|GetTargetLocation) (Variables|Default|GetCharacterLocation)) (Variables|Default|GetMinimumWarpDistance)))))

(fn AttackinCameraDirection
  (Transformation|SetActorRotation self (Math|Rotator|MakeRotator 0.0 0.0 (.yaw (Class|KismetMathLibrary|RInterptoConstant (Transformation|GetActorRotation self) (Variables|Default|GetAttackDirection) (Utilities|Time|GetWorldDeltaSeconds) 0.0))))
  (Animation|PlayAnimMontage "/Game/PaidAssets/HeroAnimations/TargetlessBasicAttack_Montage.TargetlessBasicAttack_Montage" 1.5 "None")
  (Variables|Default|SetclosestTarget 999999.0)
  (Variables|Default|Settarget 0))

(fn AttackinDirectionOfTarget
  (Transformation|SetActorRotation self (Math|Rotator|MakeRotator 0.0 0.0 (.yaw (Class|KismetMathLibrary|RInterptoConstant (Transformation|GetActorRotation self) (Math|Rotator|FindLookatRotation (Transformation|GetActorLocation self) (Transformation|GetActorLocation (Variables|Default|Gettarget))) (Utilities|Time|GetWorldDeltaSeconds) 0.0))))
  (switch int (Variables|Default|GetAttackCount)
    (:0
      (Variables|Default|SetAttackCount 1)
      (Animation|PlayAnimMontage "/Game/PaidAssets/HeroAnimations/Basic_Attack_A_Montage.Basic_Attack_A_Montage" 1.0 "None")
      (if (not (Variables|Default|GetTargetLocked))
        (Variables|Default|SetclosestTarget 999999.0)
        (Variables|Default|Settarget 0)
        (Variables|Default|SetHasTarget false)))
    (:1
      (Variables|Default|SetAttackCount 2)
      (Animation|PlayAnimMontage "/Game/PaidAssets/HeroAnimations/Basic_Attack_B_Montage.Basic_Attack_B_Montage" 1.0 "None")
      (if (not (Variables|Default|GetTargetLocked))
        (Variables|Default|SetclosestTarget 999999.0)
        (Variables|Default|Settarget 0)
        (Variables|Default|SetHasTarget false)))
    (:2
      (Variables|Default|SetAttackCount 0)
      (Animation|PlayAnimMontage "/Game/PaidAssets/HeroAnimations/Basic_Attack_C_Montage.Basic_Attack_C_Montage" 1.0 "None")
      (if (not (Variables|Default|GetTargetLocked))
        (Variables|Default|SetclosestTarget 999999.0)
        (Variables|Default|Settarget 0)
        (Variables|Default|SetHasTarget false)))))

(fn MotionWarpAttackTarget
  (Class|MotionWarpingComponent|AddorUpdateSyncPoint (Variables|Default|GetMotionWarping) "BasicAttack" (Utilities|Struct|MakeMotionWarpingSyncPoint (Variables|Default|GetTargetLocation) (Variables|Default|GetAttackDirection)))
  (switch int (Variables|Default|GetAttackCount)
    (:0
      (Variables|Default|SetAttackCount 1)
      (Animation|PlayAnimMontage "/Game/PaidAssets/HeroAnimations/Basic_Attack_Dash_A_Montage.Basic_Attack_Dash_A_Montage" 1.0 "None")
      (if (not (Variables|Default|GetTargetLocked))
        (Variables|Default|SetclosestTarget 999999.0)
        (Variables|Default|Settarget 0)
        (Variables|Default|SetHasTarget false)))
    (:1
      (Variables|Default|SetAttackCount 2)
      (Animation|PlayAnimMontage "/Game/PaidAssets/HeroAnimations/Basic_Attack_Dash_B_Montage.Basic_Attack_Dash_B_Montage" 1.0 "None")
      (if (not (Variables|Default|GetTargetLocked))
        (Variables|Default|SetclosestTarget 999999.0)
        (Variables|Default|Settarget 0)
        (Variables|Default|SetHasTarget false)))
    (:2
      (Variables|Default|SetAttackCount 0)
      (Animation|PlayAnimMontage "/Game/PaidAssets/HeroAnimations/Basic_Attack_Dash_C_Montage.Basic_Attack_Dash_C_Montage" 1.0 "None")
      (if (not (Variables|Default|GetTargetLocked))
        (Variables|Default|SetclosestTarget 999999.0)
        (Variables|Default|Settarget 0)
        (Variables|Default|SetHasTarget false)))))

(fn GetDesiredCameraRotation
  (bind _returnvalue (Utilities|Time|GetWorldDeltaSeconds))
  (bind _returnvalue_2 (Pawn|GetController))
  (bind _followcamera (Variables|Default|GetFollowCamera))
  (bind _target (Variables|Default|Gettarget))
  (bind _returnvalue_3 (Transformation|GetWorldLocation _followcamera))
  (bind _returnvalue_4 (Transformation|GetActorLocation _target))
  (bind _returnvalue_5 (Pawn|GetControlRotation _returnvalue_2 :!class /Script/Engine.Controller))
  (bind _returnvalue_6 (Math|Rotator|FindLookatRotation _returnvalue_3 _returnvalue_4))
  (bind _returnvalue_7 (Math|Interpolation|RInterpTo _returnvalue_5 _returnvalue_6 _returnvalue 5.0))
  (bind (_roll _pitch _yaw) (Math|Rotator|BreakRotator _returnvalue_7))
  (return _returnvalue_2 (Math|Rotator|MakeRotator _roll _pitch _yaw)))

(fn ResetTargetingValues
  (bind _asbp_red_enemy (Utilities|Casting|CastToBP_RedEnemy (Actor|GetParentActor (Variables|Default|Gettarget))))
  (Rendering|SetRenderCustomDepth (Variables|/Script/Engine.Character|GetMesh _asbp_red_enemy) false)
  (Variables|Default|SetTargetLocked false)
  (Variables|Default|SetclosestTarget 999999.0)
  (Variables|Default|Settarget 0)
  (Variables|Default|SetHasTarget false))